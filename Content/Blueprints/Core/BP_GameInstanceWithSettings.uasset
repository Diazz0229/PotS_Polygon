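; Game instance Blueprint that hosts and joins multiplayer sessions for the first local player controller.
; Host creates an advanced session with the given connection count and LAN flag, then opens the named level as a listen server.
; Join and accepted session invites call JoinSession directly.
; Destroy-then-end session cleanup chains lead into hosting and invite joining but are disconnected and never run.
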(event `Host`
  (params (PublicConnections :type Integer) (bUseLAN :type Boolean) (LevelName :type Name))
  ; Host Logic
  (`KismetSystemLibrary.PrintString` "HOST")
  (`CreateSessionCallbackProxyAdvanced.CreateAdvancedSession` :`PlayerController` (`GameplayStatics.GetPlayerController` 0) :`PublicConnections` PublicConnections :`bUseLAN` bUseLAN
    (:`OnSuccess`
      (`GameplayStatics.OpenLevel` LevelName false "listen"))
    (:`OnFailure`
      (`KismetSystemLibrary.PrintString` "Fail"))))

(event `Join`
  (params (SearchResult :type "BlueprintSessionResult Structure (by ref)"))
  ; Host Logic
  (`JoinSessionCallbackProxy.JoinSession` (`GameplayStatics.GetPlayerController` 0) SearchResult))

(event `self.OnSessionInviteAccepted`
  (params (LocalPlayerNum :type Integer) (PersonInvited :type "BPUniqueNetId Structure") (SessionToJoin :type "BlueprintSessionResult Structure (by ref)"))
  ; Host Logic
  (`JoinSessionCallbackProxy.JoinSession` (`GameplayStatics.GetPlayerController` 0) SessionToJoin))