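; Survival status component that models player stats such as hunger, thirst, health, sanity, stamina, temperature, radiation and toxins.
; UpdaterStart runs a looping timer that updates each entry in EffectsAdded, though only the Hunger type is dispatched so far.
; Per-stat Calculate functions scale rates by world time and modifiers, clamping results to 0–100.
; Work in progress: other calculations are uncalled here, and several regen or decay terms are multiplied by zero.
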(event `UpdaterStart`
  (params (UpdateTimeSecs :type "Float (single-precision)"))
  (`KismetSystemLibrary.K2_SetTimerDelegate` (delegate `UpdateTimer`) UpdateTimeSecs true true))

(event `UpdateTimer`
  ; Медленный апдейтер раз в секунду. Для быстрого апдейтера нужен будет другой таймер с облегченной структурой
  (for _array_element (`self.EffectsAdded`)
    (`self.StatusEffectUpdater` _array_element)))

(fn `StatusEffectUpdater`
  (params (EffectUpdated :type "/Game/Blueprints/Components/SurvivalSystem/ST_StatusEffect Structure"))
  (returns (`Success?` :type Boolean))
  (`|ExecutionSequence`
    (:`then_0`
      (switch `/Game/Blueprints/Components/SurvivalSystem/E_StatusEffect_Type` (`.Type_5_0A12976244EC9FE8CCDE09A1FC277971` (break `/Game/Blueprints/Components/SurvivalSystem/ST_StatusEffect` EffectUpdated))
        (:`NewEnumerator0`
          (`self.CalculateHunger`))))
    (:`then_1`
      (return true))))