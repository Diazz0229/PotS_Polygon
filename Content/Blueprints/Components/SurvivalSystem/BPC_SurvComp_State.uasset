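; Survival state component that tracks player vitals: health, sanity, hunger, thirst, vigor/stamina, temperature, pain shock, radiation and toxins.
; Per-stat Calculate functions scale rates by world time and update interval, apply modifiers, then clamp results.
; Vigor reads movement and sprint state from the POTS character cached on activation.
; Work in progress: several regen and decay terms are multiplied by zero, and sprint exhaustion only prints a message.
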(event `self.SurvComp_Activate`
  (bind _asbp_pots_character_base (cast `/Game/Blueprints/Core/BP_POTS_Character_BASE` (`self.ActorOwner_Ref`)))
  (set `self.POTS_Char_Ref` _asbp_pots_character_base))